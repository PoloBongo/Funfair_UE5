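; Game instance that holds the player's coin and ticket totals, giving custom events to change them.
; Add events increase the matching total by the given amount.
; Remove events subtract the amount and clamp the result at zero, so neither currency goes negative.
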(event Custom|AddCoinsToPlayer
  (params (AmountToAdd :type Integer))
  ;[1 1 1] Add Coins Event
  (Variables|Default|SetTotalCoins (+ AmountToAdd (Variables|Default|GetTotalCoins))))

(event Custom|AddTicketsToPlayer
  (params (AmountToAdd :type Integer))
  ;[1 1 1] Add Tickets Event
  (Variables|Default|SetTotalTickets (+ AmountToAdd (Variables|Default|GetTotalTickets))))

(event Custom|RemoveCoinsToPlayer
  (params (Amount%20To%20Remove :type Integer))
  ;[1 1 1] Remove Coins Event
  (if (> (- (Variables|Default|GetTotalCoins) Amount%20To%20Remove) 0)
    (Variables|Default|SetTotalCoins (- (Variables|Default|GetTotalCoins) Amount%20To%20Remove))
    (else
      (Variables|Default|SetTotalCoins 0))))

(event Custom|RemoveTicketsToPlayer
  (params (AmountToRemove :type Integer))
  ;[1 1 1] Remove Tickets Event
  (if (> (- (Variables|Default|GetTotalTickets) AmountToRemove) 0)
    (Variables|Default|SetTotalTickets (- (Variables|Default|GetTotalTickets) AmountToRemove))
    (else
      (Variables|Default|SetTotalTickets 0))))