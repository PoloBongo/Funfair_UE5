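; BP_ManageCoins tracks the player's two currencies, coins and tickets, and puts the player HUD on screen.
; On BeginPlay it creates the WG_Player widget, adds it to the viewport and grants a starting balance of both currencies.
; Add and Remove events adjust TotalCoins and TotalTickets, with removal clamped at zero rather than rejecting overspending.
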(event Custom|AddCoinsToPlayer
  (params (AmountToAdd :type Integer))
  (Variables|Default|SetTotalCoins (+ AmountToAdd (Variables|Default|GetTotalCoins))))

(event Custom|AddTicketsToPlayer
  (params (AmountToAdd :type Integer))
  (Variables|Default|SetTotalTickets (+ AmountToAdd (Variables|Default|GetTotalTickets))))

(event Custom|RemoveCoinsToPlayer
  (params (Amount%20To%20Remove :type Integer))
  (if (> (- (Variables|Default|GetTotalCoins) Amount%20To%20Remove) 0)
    (Variables|Default|SetTotalCoins (- (Variables|Default|GetTotalCoins) Amount%20To%20Remove))
    (else
      (Variables|Default|SetTotalCoins 0))))

(event Custom|RemoveTicketsToPlayer
  (params (AmountToRemove :type Integer))
  (if (> (- (Variables|Default|GetTotalTickets) AmountToRemove) 0)
    (Variables|Default|SetTotalTickets (- (Variables|Default|GetTotalTickets) AmountToRemove))
    (else
      (Variables|Default|SetTotalTickets 0))))

(event EventBeginPlay
  (bind _returnvalue (Game|ConstructObjectfromClass "/Game/Blueprints/Player/WG_Player.WG_Player_C"))
  (bind _output_get (Variables|Default|SetWG_Player _returnvalue))
  (UserInterface|Viewport|AddtoViewport _output_get 0)
  (CallFunction|AddCoinstoPlayer 100)
  (CallFunction|AddTicketstoPlayer 10))

(fn ConstructionScript)