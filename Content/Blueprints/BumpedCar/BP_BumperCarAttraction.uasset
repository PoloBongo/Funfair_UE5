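; Bumper car attraction actor that moves the player into a bumper car when its start trigger is overlapped.
; On overlap it teleports the player pawn to a set position, stops character movement and adds the bumper car Enhanced Input mapping context.
; The player controller then possesses a random BP_PawnBumperCar found in the level.
; The overlap does not check which actor entered, and no exit logic is present.
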(event OnComponentBeginOverlap(StartTrigger)
  (params (OverlappedComponent :type Primitive%20Component%20Object%20Reference) (OtherActor :type Actor%20Object%20Reference) (OtherComp :type Primitive%20Component%20Object%20Reference) (OtherBodyIndex :type Integer) (bFromSweep :type Boolean) (SweepResult :type Hit%20Result%20Structure%20%28by%20ref%29))
  (Transformation|SetActorLocation (Game|Player|GetPlayerPawn 0) (Variables|Default|GetTeleportPos) false true)
  (Components|Movement|StopMovementImmediately (Variables|/Script/Engine.Character|GetCharacterMovement (Game|GetPlayerCharacter 0)))
  (Input|AddMappingContext (PlayerController|LocalPlayerSubsystems|GetEnhancedInputLocalPlayerSubsystem (Game|GetPlayerController 0)) "/Game/Inputs/BumpedCar/IMC_BumpedCar.IMC_BumpedCar" 0 "(bIgnoreAllPressedKeysUntilRelease=True,bForceImmediately=False,bNotifyUserSettings=False)")
  (bind _outactors (Actor|GetAllActorsOfClass "/Game/Blueprints/BumpedCar/BP_PawnBumperCar.BP_PawnBumperCar_C"))
  (Pawn|Possess (Game|GetPlayerController 0) (.OutItem (Utilities|Array|Random _outactors))))

(fn ConstructionScript)