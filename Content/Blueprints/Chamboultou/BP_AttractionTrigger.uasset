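; Fairground trigger for the Chamboule Tout knock-down minigame, played for one ticket when the player presses E inside it.
; It blends to the attraction camera, swaps movement for BP_ShootBehaviour and shows a widget with a mouse-following crosshair.
; rFunction counts shots, while BoxesTrigger counts fallen BP_ChamboulTout actors to detect a win.
; Endings restore camera and controls, reinitialise targets, notify in French and award coins on a win.
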(event OnComponentBeginOverlap(StartTrigger)
  (params (OverlappedComponent :type Primitive%20Component%20Object%20Reference) (OtherActor :type Actor%20Object%20Reference) (OtherComp :type Primitive%20Component%20Object%20Reference) (OtherBodyIndex :type Integer) (bFromSweep :type Boolean) (SweepResult :type Hit%20Result%20Structure%20%28by%20ref%29))
  (bind _asbp_third_person_character (Utilities|Casting|CastToBP_ThirdPersonCharacter OtherActor))
  (Variables|Default|SetplayerInTrigger true)
  (Variables|Default|SetMy%20Third%20Person%20Character _asbp_third_person_character)
  (bind _returnvalue (Actor|GetActorOfClass "/Game/Blueprints/Player/BP_NotificationPush.BP_NotificationPush_C"))
  (Variables|Default|SetBP_Notification _returnvalue))

(event OnComponentBeginOverlap(BoxesTrigger)
  (params (OverlappedComponent :type Primitive%20Component%20Object%20Reference) (OtherActor :type Actor%20Object%20Reference) (OtherComp :type Primitive%20Component%20Object%20Reference) (OtherBodyIndex :type Integer) (bFromSweep :type Boolean) (SweepResult :type Hit%20Result%20Structure%20%28by%20ref%29))
  (Utilities|Casting|CastToBP_ChamboulTout OtherActor)
  (bind _output_get (Variables|Default|SetBallsFallen (+ 1 (Variables|Default|GetBallsFallen))))
  (if (== _output_get (Variables|Default|GettotalBoite))
    (Variables|Default|SethasWin true)
    (Default|NotificationPushEvent (Variables|Default|GetBP_Notification) "Tu viens de gagner au Chamboule Tout!" (Utilities|Struct|MakeSlateColor "(R=0.110319,G=1.000000,B=0.000000,A=1.000000)"))
    (Variables|/Game/Blueprints/Chamboultou/BP_ShootBehaviour.BP_ShootBehaviour_C|SetcanShoot (Variables|Default|GetShootBehavior) false)
    (Utilities|FlowControl|Delay 2.0)
    (Game|Player|SetViewTargetwithBlend (Game|GetPlayerController 0) (Components|GetOwner (Variables|/Game/ThirdPerson/Blueprints/BP_ThirdPersonCharacter.BP_ThirdPersonCharacter_C|GetFollowCamera (Variables|Default|GetMy%20Third%20Person%20Character))) 2.0 "VTBlend_Linear" 0.0 false)
    (if (Variables|Default|GethasWin)
      (bind _asmy_game_instance (Utilities|Casting|CastToMyGameInstance (Game|GetGameInstance)))
      (Default|AddCoinstoPlayer _asmy_game_instance 50)
      (else
        (Default|NotificationPushEvent (Variables|Default|GetBP_Notification) "Tu viens de perdre au Chamboule Tout!" (Utilities|Struct|MakeSlateColor "(R=1.000000,G=0.037472,B=0.000000,A=1.000000)"))
        (Utilities|FlowControl|Delay 2.0)))
    (CallFunction|EndGameEvent)
    (bind _outactors (Actor|GetAllActorsOfClass "/Game/Blueprints/Chamboultou/BP_ChamboulTout.BP_ChamboulTout_C"))
    (for _array_element _outactors
      (Default|Reinit _array_element)
      (Widget|RemovefromParent (stale Custom|ReadyToPlayChamboultout _returnvalue_2)))))

(event OnComponentEndOverlap(StartTrigger)
  (params (OverlappedComponent :type Primitive%20Component%20Object%20Reference) (OtherActor :type Actor%20Object%20Reference) (OtherComp :type Primitive%20Component%20Object%20Reference) (OtherBodyIndex :type Integer))
  (Variables|Default|SetplayerInGame false)
  (Variables|Default|SetNotification "")
  (Variables|Default|SetplayerInTrigger false))

(event Custom|ReadyToPlayChamboultout
  (bind _my_third_person_character (Variables|Default|GetMy%20Third%20Person%20Character))
  (bind _returnvalue (Actor|GetComponentbyClass _my_third_person_character "/Game/Blueprints/Chamboultou/BP_ShootBehaviour.BP_ShootBehaviour_C"))
  (Variables|Default|SetShootBehavior _returnvalue)
  (Variables|/Game/Blueprints/Chamboultou/BP_ShootBehaviour.BP_ShootBehaviour_C|SetCameraAttraction _returnvalue (Variables|Default|GetCamera))
  (Components|Activation|SetActive _returnvalue true false)
  (Components|Activation|SetActive (Actor|GetComponentbyClass _my_third_person_character "/Script/Engine.CharacterMovementComponent") false false)
  (bind _returnvalue_2 (Game|ConstructObjectfromClass (Game|GetPlayerController 0) "/Game/Blueprints/Chamboultou/WG_Chamboultout.WG_Chamboultout_C"))
  (Variables|/Game/Blueprints/Chamboultou/WG_Chamboultout.WG_Chamboultout_C|Setattraction _returnvalue_2 self)
  (UserInterface|Viewport|AddtoViewport _returnvalue_2 0)
  (Variables|Default|SetCrosshair (Variables|/Game/Blueprints/Chamboultou/WG_Chamboultout.WG_Chamboultout_C|GetCrosshair _returnvalue_2))
  (Variables|Default|SetsetupFinish true)
  (Variables|/Game/Blueprints/Chamboultou/BP_ShootBehaviour.BP_ShootBehaviour_C|SetcanShoot (Variables|Default|GetShootBehavior) true))

(event EventrFunction
  (bind _output_get (Variables|Default|SetactualShoot (+ 1 (Variables|Default|GetactualShoot))))
  (if (== _output_get (Variables|Default|GetmaxShoot))
    (Utilities|FlowControl|Delay 1.0)
    (Game|Player|SetViewTargetwithBlend (Game|GetPlayerController 0) (Components|GetOwner (Variables|/Game/ThirdPerson/Blueprints/BP_ThirdPersonCharacter.BP_ThirdPersonCharacter_C|GetFollowCamera (Variables|Default|GetMy%20Third%20Person%20Character))) 2.0 "VTBlend_Linear" 0.0 false)
    (if (Variables|Default|GethasWin)
      (bind _asmy_game_instance (Utilities|Casting|CastToMyGameInstance (Game|GetGameInstance)))
      (Default|AddCoinstoPlayer _asmy_game_instance 50)
      (else
        (Default|NotificationPushEvent (Variables|Default|GetBP_Notification) "Tu viens de perdre au Chamboule Tout!" (Utilities|Struct|MakeSlateColor "(R=1.000000,G=0.037472,B=0.000000,A=1.000000)"))
        (Utilities|FlowControl|Delay 2.0)))
    (CallFunction|EndGameEvent)
    (bind _outactors (Actor|GetAllActorsOfClass "/Game/Blueprints/Chamboultou/BP_ChamboulTout.BP_ChamboulTout_C"))
    (for _array_element _outactors
      (Default|Reinit _array_element)
      (Widget|RemovefromParent (stale Custom|ReadyToPlayChamboultout _returnvalue_2)))))

(event EventTick
  (params (DeltaSeconds :type Float%20%28single-precision%29))
  (bind _returnvalue (Game|GetPlayerController 0))
  (bind (_locationx _locationy) (Game|Player|GetMousePosition _returnvalue))
  (if (Variables|Default|GetsetupFinish)
    (Class|CanvasPanelSlot|SetPosition (Class|WidgetLayoutLibrary|SlotasCanvasSlot (Variables|Default|GetCrosshair)) (Class|SlateBlueprintLibrary|ScreentoViewport (Math|Vector2D|MakeVector2D _locationx _locationy)))))

(event Input|KeyboardEvents|E
  (params (Key :type Key%20Structure :default "None"))
  (:Pressed
    (if (Variables|Default|GetplayerInTrigger)
      (if (not (Variables|Default|GetplayerInGame))
        (Variables|Default|SetplayerInGame true)
        (bind _returnvalue (Actor|GetActorOfClass "/Game/Blueprints/Player/BP_ManageCoins.BP_ManageCoins_C"))
        (Widget|SetVisibility (Variables|/Game/Blueprints/Player/BP_ManageCoins.BP_ManageCoins_C|GetWG_Player _returnvalue) "Hidden")
        (bind _asmy_game_instance (Utilities|Casting|CastToMyGameInstance (Game|GetGameInstance)))
        (if (> (Variables|/Game/Blueprints/Player/MyGameInstance.MyGameInstance_C|GetTotalTickets _asmy_game_instance) 0)
          (bind _returnvalue_2 (Actor|GetActorOfClass "/Game/Blueprints/Chamboultou/UI/BP_UIWorldSpace.BP_UIWorldSpace_C"))
          (Default|DisplayWorldSpaceText _returnvalue_2 false)
          (bind _asmy_game_instance_2 (Utilities|Casting|CastToMyGameInstance (Game|GetGameInstance)))
          (Default|RemoveTicketstoPlayer _asmy_game_instance_2 1)
          (Variables|Default|SetTextEndGame "")
          (Variables|Default|SetactualShoot 0)
          (Variables|Default|SetBallsFallen 0)
          (Game|Player|SetViewTargetwithBlend (Game|GetPlayerController 0) (Components|GetOwner (Variables|Default|GetCamera)) 1.0 "VTBlend_Linear" 0.0 false)
          (Utilities|FlowControl|Delay 1.0)
          (CallFunction|ReadytoPlayChamboultout)
          (else
            (Default|NotificationPushEvent (Variables|Default|GetBP_Notification) "Vous n'avez pas assez de tickets pour faire cette attraction!" (Utilities|Struct|MakeSlateColor "(R=1.000000,G=0.047017,B=0.000000,A=1.000000)"))))))))

(event Custom|EndGameEvent
  (bind _my_third_person_character (Variables|Default|GetMy%20Third%20Person%20Character))
  (bind _returnvalue (Actor|GetComponentbyClass _my_third_person_character "/Game/Blueprints/Chamboultou/BP_ShootBehaviour.BP_ShootBehaviour_C"))
  (Variables|/Game/Blueprints/Chamboultou/BP_ShootBehaviour.BP_ShootBehaviour_C|SetCameraAttraction _returnvalue (Variables|Default|GetCamera))
  (Components|Activation|SetActive _returnvalue false false)
  (Components|Activation|SetActive (Actor|GetComponentbyClass _my_third_person_character "/Script/Engine.CharacterMovementComponent") true false)
  (bind _returnvalue_2 (Actor|GetActorOfClass "/Game/Blueprints/Chamboultou/UI/BP_UIWorldSpace.BP_UIWorldSpace_C"))
  (Default|DisplayWorldSpaceText _returnvalue_2 true)
  (Variables|Default|SetplayerInGame false)
  (bind _returnvalue_3 (Actor|GetActorOfClass "/Game/Blueprints/Player/BP_ManageCoins.BP_ManageCoins_C"))
  (Widget|SetVisibility (Variables|/Game/Blueprints/Player/BP_ManageCoins.BP_ManageCoins_C|GetWG_Player _returnvalue_3) "Visible")
  (Variables|Default|SetNotification ""))

(fn ConstructionScript)