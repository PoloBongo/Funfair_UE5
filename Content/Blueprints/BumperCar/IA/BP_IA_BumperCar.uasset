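; AI bumper car NPC that wanders between BP_AI_TargetPoint actors and sometimes chases the third-person character.
; On BeginPlay it caches the points and character, then loops AIMoveTo to a random point, waits a random delay, and either moves again or chases, depending on the point's type.
; The chase picks a random bumper car but targets the character, then resumes wandering on success; failed moves are not handled.
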(event Custom|MoveNPC
  (bind _returnvalue (Math|Random|RandomFloatinRange 2.0 6.0))
  ;[1 1 1] Move NPC to a random target point
  (bind _output_get (Variables|Default|SetCurTargetPoint (.OutItem (Utilities|Array|Random (Variables|Default|GetOut%20Actors)))))
  (AI|AIMoveTo self (.RandomLocation (AI|Navigation|GetRandomReachablePointinRadius (Transformation|GetActorLocation _output_get) 0.0 0 0)) 0 5.0 false
    (:OnSuccess
      (switch Utilities|FlowControl|Switch|SwitchonE_NavChaseType (Variables|/Game/Blueprints/BumperCar/IA/BP_AI_TargetPoint.BP_AI_TargetPoint_C|GetType (Variables|Default|GetCurTargetPoint))
        (:NewEnumerator0
          (Utilities|FlowControl|Delay _returnvalue)
          (CallFunction|MoveNPC))
        (:NewEnumerator1
          (Utilities|FlowControl|Delay _returnvalue)
          (CallFunction|ChaseBumperCar))))))

(event Custom|ChaseBumperCar
  (bind _bp_thirdcharacter (Variables|Default|GetBP_ThirdCharacter))
  ;[1 1 1] Move NPC to a random target point
  (bind _outactors (Actor|GetAllActorsOfClass "/Game/Blueprints/BumperCar/BP_PawnBumperCar.BP_PawnBumperCar_C"))
  (Variables|Default|SetCur%20Target%20Bumper%20Car (.OutItem (Utilities|Array|Random _outactors)))
  (AI|AIMoveTo self (.RandomLocation (AI|Navigation|GetRandomReachablePointinRadius (Transformation|GetActorLocation _bp_thirdcharacter) 0.0 0 0)) _bp_thirdcharacter 0.0 false
    (:OnSuccess
      (CallFunction|MoveNPC))))

(event EventBeginPlay
  ;[1 1 1] Récupère tout les targets points pour pouvoir s'y rendre plus tard
  (bind _outactors (Actor|GetAllActorsOfClass "/Game/Blueprints/BumperCar/IA/BP_AI_TargetPoint.BP_AI_TargetPoint_C"))
  (Variables|Default|SetOut%20Actors _outactors)
  (bind _returnvalue (Actor|GetActorOfClass "/Game/ThirdPerson/Blueprints/BP_ThirdPersonCharacter.BP_ThirdPersonCharacter_C"))
  (Variables|Default|SetBP_ThirdCharacter _returnvalue)
  (CallFunction|MoveNPC))

(fn ConstructionScript)