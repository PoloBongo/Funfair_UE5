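; Bumper car light rig that moves an array of actors around a spline, likely as moving lights for the bumper car attraction.
; A timeline drives evenly offset actors along the spline, wrapping at its end and fixing pitch at -90.
; Each cycle restarts at a random play rate, recolors all lights randomly and randomly hides some of the first few.
; The construction script pre-places the actors along the spline.
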(event Custom|PlayTimeLine
  (bind _spline (Variables|Default|GetSpline))
  (bind _spline_2 (Variables|Default|GetSpline))
  (bind _returnvalue (Spline|GetSplineLength _spline))
  (bind _alpha (Timeline|Timeline PlayFromStart)
    (:Update
      (for (_array_element _array_index) (Variables|Default|GetActors)
        (bind _output_get (Variables|Default|SetDistanceAlongSpline (+ (Math|Float|Lerp 0.0 (Spline|GetSplineLength (Variables|Default|GetSpline)) _alpha) (* _array_index (Variables|Default|GetOffsetbetweenActors)))))
        (if (> _output_get _returnvalue)
          (Variables|Default|SetDistanceAlongSpline (- (Variables|Default|GetDistanceAlongSpline) _returnvalue)))
        (Transformation|SetActorLocationAndRotation _array_element (Spline|GetLocationatDistanceAlongSpline _spline_2 (Variables|Default|GetDistanceAlongSpline) "World") (Math|Rotator|MakeRotator (.roll (Spline|GetRotationatDistanceAlongSpline _spline_2 (Variables|Default|GetDistanceAlongSpline) "World")) -9e+01 (.yaw (Spline|GetRotationatDistanceAlongSpline _spline_2 (Variables|Default|GetDistanceAlongSpline) "World"))))))
    (:Finished
      (CallFunction|Init)
      (CallFunction|PlayTimeLine)
      (for (_array_element_2 _array_index_2) (Variables|Default|GetAllLights)
        (Rendering|Components|Light|SetLightColor (Variables|/Script/Engine.Light|GetLightComponent _array_element_2) (Utilities|Struct|MakeLinearColor (Math|Random|RandomFloatinRange 0.0 1.0) (Math|Random|RandomFloatinRange 0.0 1.0) (Math|Random|RandomFloatinRange 0.0 1.0) 1.0) true)
        (if (> _array_index_2 (Math|Random|RandomInteger 3))
          (Rendering|SetVisibility (Variables|/Script/Engine.Light|GetLightComponent _array_element_2) true false)
          (else
            (Rendering|SetVisibility (Variables|/Script/Engine.Light|GetLightComponent _array_element_2) false false)))))))

(event Custom|Init
  (Components|Timeline|SetPlayRate (Variables|Default|GetTimeline) (/ 1.0 (Math|Random|RandomFloatinRange (Variables|Default|GetTimelineLength) 5.0)))
  (CallFunction|PlayTimeLine))

(event EventBeginPlay
  (CallFunction|Init))

(fn ConstructionScript
  (bind _spline (Variables|Default|GetSpline))
  (for (_array_element _array_index) (Variables|Default|GetActors)
    (Transformation|SetActorLocationAndRotation _array_element (Spline|GetLocationatDistanceAlongSpline _spline (* (Variables|Default|GetOffsetbetweenActors) _array_index) "World") (Spline|GetRotationatDistanceAlongSpline _spline (* (Variables|Default|GetOffsetbetweenActors) _array_index) "World"))))