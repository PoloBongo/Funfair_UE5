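; BP_PawnBumperCar is a player-driven bumper car pawn steered through Enhanced Input move and turn actions.
; The move action applies physics force along the static mesh's forward vector, scaled by input value and MassForce.
; The turn action directly sets the mesh's rotation by combining a yaw step from input and TurnSpeed with its current rotation, without delta-time scaling.
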(event Input|EnhancedActionEvents|EnhancedInputActionIA_BumpedCarMove
  (params (ActionValue :type Float%20%28double-precision%29) (ElapsedSeconds :type Float%20%28double-precision%29) (TriggeredSeconds :type Float%20%28double-precision%29) (InputAction :type Input%20Action%20Object%20Reference :default "/Game/Inputs/BumpedCar/IA_BumpedCarMove.IA_BumpedCarMove"))
  (Physics|AddForce (Variables|Default|GetStaticMesh) (* (* (Variables|Default|GetmassForce) ActionValue) (Math|Vector|GetForwardVector (Variables|Default|GetStaticMesh))) "None" false))

(event Input|EnhancedActionEvents|EnhancedInputActionIA_BumpedCarTurn
  (params (ActionValue :type Float%20%28double-precision%29) (ElapsedSeconds :type Float%20%28double-precision%29) (TriggeredSeconds :type Float%20%28double-precision%29) (InputAction :type Input%20Action%20Object%20Reference :default "/Game/Inputs/BumpedCar/IA_BumpedCarTurn.IA_BumpedCarTurn"))
  (Transformation|SetWorldRotation (Variables|Default|GetStaticMesh) (Math|Rotator|CombineRotators (Math|Rotator|MakeRotator 0.0 0.0 (* ActionValue (Variables|Default|GetTurnSpeed))) (Transformation|GetWorldRotation (Variables|Default|GetStaticMesh))) false false))

(fn ConstructionScript)