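; Bumper car minigame attraction: pressing E in the start trigger spends a ticket and possesses a random BP_PawnBumperCar with its own input context and HUD.
; Defeat triggers count rival cars knocked out, paying coins for each until the maximum; that or the player's exit (ignored by DefeatTrigger2) stops the HUD timer.
; BumperCarEndGame announces win or loss, restores the original pawn and input, and resets the cars.
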(event OnComponentBeginOverlap(StartTrigger)
  (params (OverlappedComponent :type Primitive%20Component%20Object%20Reference) (OtherActor :type Actor%20Object%20Reference) (OtherComp :type Primitive%20Component%20Object%20Reference) (OtherBodyIndex :type Integer) (bFromSweep :type Boolean) (SweepResult :type Hit%20Result%20Structure%20%28by%20ref%29))
  (bind _asbp_third_person_character (Utilities|Casting|CastToBP_ThirdPersonCharacter OtherActor))
  (Variables|Default|SetAs%20BP%20Third%20Person%20Character _asbp_third_person_character)
  (Variables|Default|SetplayerInTrigger true)
  (bind _returnvalue (Actor|GetActorOfClass "/Game/Blueprints/Player/BP_NotificationPush.BP_NotificationPush_C"))
  (Variables|Default|SetBP_Notification _returnvalue))

(event OnComponentBeginOverlap(DefeatTrigger)
  (params (OverlappedComponent :type Primitive%20Component%20Object%20Reference) (OtherActor :type Actor%20Object%20Reference) (OtherComp :type Primitive%20Component%20Object%20Reference) (OtherBodyIndex :type Integer) (bFromSweep :type Boolean) (SweepResult :type Hit%20Result%20Structure%20%28by%20ref%29))
  (bind _asbp_pawn_bumper_car (Utilities|Casting|CastToBP_PawnBumperCar OtherActor))
  (if (== _asbp_pawn_bumper_car (Variables|Default|GetSaveBP_PawnBumperCar))
    (Default|StopUpdateTimer (Variables|Default|GetWG_BumperCar) true)
    (else
      (CallFunction|CheckCarOut))))

(event OnComponentBeginOverlap(DefeatTrigger2)
  (params (OverlappedComponent :type Primitive%20Component%20Object%20Reference) (OtherActor :type Actor%20Object%20Reference) (OtherComp :type Primitive%20Component%20Object%20Reference) (OtherBodyIndex :type Integer) (bFromSweep :type Boolean) (SweepResult :type Hit%20Result%20Structure%20%28by%20ref%29))
  (bind _asbp_pawn_bumper_car (Utilities|Casting|CastToBP_PawnBumperCar OtherActor))
  (if (not (== _asbp_pawn_bumper_car (Variables|Default|GetSaveBP_PawnBumperCar)))
    (CallFunction|CheckCarOut)))

(event OnComponentBeginOverlap(DefeatTrigger3)
  (params (OverlappedComponent :type Primitive%20Component%20Object%20Reference) (OtherActor :type Actor%20Object%20Reference) (OtherComp :type Primitive%20Component%20Object%20Reference) (OtherBodyIndex :type Integer) (bFromSweep :type Boolean) (SweepResult :type Hit%20Result%20Structure%20%28by%20ref%29))
  (bind _asbp_pawn_bumper_car (Utilities|Casting|CastToBP_PawnBumperCar OtherActor))
  (if (== _asbp_pawn_bumper_car (Variables|Default|GetSaveBP_PawnBumperCar))
    (Default|StopUpdateTimer (Variables|Default|GetWG_BumperCar) true)
    (else
      (CallFunction|CheckCarOut))))

(event Custom|CheckCarOut
  (bind _output_get (Variables|Default|SetNumberOfBumperCarOut (+ (Variables|Default|GetNumberOfBumperCarOut) 1)))
  (if (== _output_get (Variables|Default|GetmaxBumperCarInAttraction))
    (Default|StopUpdateTimer (Variables|Default|GetWG_BumperCar) false)
    (else
      (Default|AddCoinstoPlayer (Variables|Default|GetManageCoins) 5)
      (bind _returnvalue (Actor|GetActorOfClass "/Game/Blueprints/Player/BP_NotificationPush.BP_NotificationPush_C"))
      (Default|NotificationPushEvent _returnvalue "Une auto-tamponneuse est sortie! +5 coins" (Utilities|Struct|MakeSlateColor "(R=0.000000,G=0.772792,B=1.000000,A=1.000000)")))))

(event Input|KeyboardEvents|E
  (params (Key :type Key%20Structure :default "None"))
  (bind _returnvalue (Game|GetPlayerController 0))
  (bind _returnvalue_2 (PlayerController|LocalPlayerSubsystems|GetEnhancedInputLocalPlayerSubsystem _returnvalue))
  (:Pressed
    (if (not (Variables|Default|GetIsEnter))
      (if (Variables|Default|GetplayerInTrigger)
        (Variables|Default|SetIsEnter true)
        (bind _returnvalue_3 (Actor|GetActorOfClass "/Game/Blueprints/Player/BP_ManageCoins.BP_ManageCoins_C"))
        (Variables|Default|SetManageCoins _returnvalue_3)
        (if (> (Variables|/Game/Blueprints/Player/BP_ManageCoins.BP_ManageCoins_C|GetTotalTickets _returnvalue_3) 0)
          (Default|RemoveTicketstoPlayer (Variables|Default|GetManageCoins) 1)
          (bind _output_get (Variables|Default|SetWG%20Player (Variables|/Game/Blueprints/Player/BP_ManageCoins.BP_ManageCoins_C|GetWG_Player _returnvalue_3)))
          (Widget|SetVisibility _output_get "Hidden")
          (Variables|Default|SetNumberOfBumperCarOut 0)
          (Variables|Default|SetnameBumperCar "")
          (bind _returnvalue_4 (Game|ConstructObjectfromClass "/Game/Blueprints/BumperCar/WG_BumperCar.WG_BumperCar_C"))
          (Variables|/Game/Blueprints/BumperCar/WG_BumperCar.WG_BumperCar_C|SetBP_BumperCarAttraction _returnvalue_4 self)
          (bind _output_get_2 (Variables|Default|SetWG_BumperCar _returnvalue_4))
          (UserInterface|Viewport|AddtoViewport _output_get_2 0)
          (bind _output_get_3 (Variables|Default|SetSaveOriginalPlayerPawn (Game|Player|GetPlayerPawn 0)))
          (Transformation|SetActorLocation _output_get_3 (Variables|Default|GetTeleportPos) false true)
          (Components|Movement|StopMovementImmediately (Variables|/Script/Engine.Character|GetCharacterMovement (Game|GetPlayerCharacter 0)))
          (Input|RemoveMappingContext _returnvalue_2 "/Game/ThirdPerson/Input/IMC_Default.IMC_Default" "(bIgnoreAllPressedKeysUntilRelease=True,bForceImmediately=False,bNotifyUserSettings=False)")
          (Input|AddMappingContext _returnvalue_2 "/Game/Inputs/BumpedCar/IMC_BumpedCar.IMC_BumpedCar" 1 "(bIgnoreAllPressedKeysUntilRelease=True,bForceImmediately=False,bNotifyUserSettings=False)")
          (bind _outactors (Actor|GetAllActorsOfClass "/Game/Blueprints/BumperCar/BP_PawnBumperCar.BP_PawnBumperCar_C"))
          (bind _output_get_4 (Variables|Default|SetSaveBP_PawnBumperCar (.OutItem (Utilities|Array|Random _outactors))))
          (Variables|Default|SetnameBumperCar (Utilities|GetDisplayName _output_get_4))
          (Pawn|Possess (Game|GetPlayerController 0) _output_get_4)
          (Variables|Default|SetIsEnter true)
          (else
            (Default|NotificationPushEvent (Variables|Default|GetBP_Notification) "Vous n'avez pas assez de tickets pour faire cette attraction!" (Utilities|Struct|MakeSlateColor "(R=1.000000,G=0.006526,B=0.000000,A=1.000000)"))))))))

(event Custom|BumperCarEndGame
  (params (isWin :type Boolean))
  (bind _returnvalue (Game|GetPlayerController 0))
  (bind _returnvalue_2 (Game|GetPlayerController 0))
  (bind _returnvalue_3 (PlayerController|LocalPlayerSubsystems|GetEnhancedInputLocalPlayerSubsystem _returnvalue_2))
  (if isWin
    (Default|NotificationPushEvent (Variables|Default|GetBP_Notification) "Vous avez gagné!" (Utilities|Struct|MakeSlateColor "(R=0.011553,G=1.000000,B=0.000000,A=1.000000)"))
    (else
      (Default|NotificationPushEvent (Variables|Default|GetBP_Notification) "Vous avez perdu!" (Utilities|Struct|MakeSlateColor "(R=1.000000,G=0.006526,B=0.000000,A=1.000000)"))))
  (Input|RemoveMappingContext _returnvalue_3 "/Game/Inputs/BumpedCar/IMC_BumpedCar.IMC_BumpedCar" "(bIgnoreAllPressedKeysUntilRelease=True,bForceImmediately=False,bNotifyUserSettings=False)")
  (Input|AddMappingContext _returnvalue_3 "/Game/ThirdPerson/Input/IMC_Default.IMC_Default" 1 "(bIgnoreAllPressedKeysUntilRelease=True,bForceImmediately=False,bNotifyUserSettings=False)")
  (Pawn|UnPossess _returnvalue)
  (Pawn|Possess _returnvalue (Variables|Default|GetSaveOriginalPlayerPawn))
  (Game|Player|SetViewTargetwithBlend (Game|GetPlayerController 0) (Variables|Default|GetAs%20BP%20Third%20Person%20Character) 1.0 "VTBlend_Linear" 0.0 false)
  (bind _outactors (Actor|GetAllActorsOfClass "/Game/Blueprints/BumperCar/BP_PawnBumperCar.BP_PawnBumperCar_C"))
  (for _array_element _outactors
    (Default|ReInitBumperCar _array_element)
    (Utilities|FlowControl|Delay 4.0)
    (Variables|Default|SetIsEnter false)
    (Variables|Default|SetSetEndGameText "")
    (Widget|RemovefromParent (Variables|Default|GetWG_BumperCar))
    (Widget|SetVisibility (Variables|Default|GetWG%20Player) "Visible")))

(fn ConstructionScript)