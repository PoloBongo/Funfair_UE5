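; Ticketed roller coaster ride: pressing E in range spends a ticket, disables default input and blends the view to the car.
; A timeline moves an array of actors along a spline at index-based offsets, which the construction script also uses for initial placement.
; Slow and speed trigger overlaps by the car change the timeline's play rate.
; When the timeline finishes, view and input return, coins are awarded and a notification shows.
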(event OnComponentBeginOverlap(SlowTrigger)
  (params (OverlappedComponent :type Primitive%20Component%20Object%20Reference) (OtherActor :type Actor%20Object%20Reference) (OtherComp :type Primitive%20Component%20Object%20Reference) (OtherBodyIndex :type Integer) (bFromSweep :type Boolean) (SweepResult :type Hit%20Result%20Structure%20%28by%20ref%29))
  (Utilities|Casting|CastToBP_CarRollerCoaster OtherActor)
  (CallFunction|SlowEvent 6e+01))

(event OnComponentBeginOverlap(SpeedTrigger)
  (params (OverlappedComponent :type Primitive%20Component%20Object%20Reference) (OtherActor :type Actor%20Object%20Reference) (OtherComp :type Primitive%20Component%20Object%20Reference) (OtherBodyIndex :type Integer) (bFromSweep :type Boolean) (SweepResult :type Hit%20Result%20Structure%20%28by%20ref%29))
  (Utilities|Casting|CastToBP_CarRollerCoaster OtherActor)
  (CallFunction|SpeedEvent 25.0))

(event OnComponentBeginOverlap(SpeedTrigger1)
  (params (OverlappedComponent :type Primitive%20Component%20Object%20Reference) (OtherActor :type Actor%20Object%20Reference) (OtherComp :type Primitive%20Component%20Object%20Reference) (OtherBodyIndex :type Integer) (bFromSweep :type Boolean) (SweepResult :type Hit%20Result%20Structure%20%28by%20ref%29))
  (Utilities|Casting|CastToBP_CarRollerCoaster OtherActor)
  (CallFunction|SpeedEvent 3e+01))

(event OnComponentBeginOverlap(SlowTrigger1)
  (params (OverlappedComponent :type Primitive%20Component%20Object%20Reference) (OtherActor :type Actor%20Object%20Reference) (OtherComp :type Primitive%20Component%20Object%20Reference) (OtherBodyIndex :type Integer) (bFromSweep :type Boolean) (SweepResult :type Hit%20Result%20Structure%20%28by%20ref%29))
  (Utilities|Casting|CastToBP_CarRollerCoaster OtherActor)
  (CallFunction|SlowEvent 4e+01))

(event OnComponentBeginOverlap(SlowTrigger2)
  (params (OverlappedComponent :type Primitive%20Component%20Object%20Reference) (OtherActor :type Actor%20Object%20Reference) (OtherComp :type Primitive%20Component%20Object%20Reference) (OtherBodyIndex :type Integer) (bFromSweep :type Boolean) (SweepResult :type Hit%20Result%20Structure%20%28by%20ref%29))
  (Utilities|Casting|CastToBP_CarRollerCoaster OtherActor)
  (CallFunction|SlowEvent 4e+01))

(event OnComponentBeginOverlap(SlowTrigger3)
  (params (OverlappedComponent :type Primitive%20Component%20Object%20Reference) (OtherActor :type Actor%20Object%20Reference) (OtherComp :type Primitive%20Component%20Object%20Reference) (OtherBodyIndex :type Integer) (bFromSweep :type Boolean) (SweepResult :type Hit%20Result%20Structure%20%28by%20ref%29))
  (Utilities|Casting|CastToBP_CarRollerCoaster OtherActor)
  (CallFunction|SlowEvent 6e+01))

(event OnComponentBeginOverlap(SlowTrigger4)
  (params (OverlappedComponent :type Primitive%20Component%20Object%20Reference) (OtherActor :type Actor%20Object%20Reference) (OtherComp :type Primitive%20Component%20Object%20Reference) (OtherBodyIndex :type Integer) (bFromSweep :type Boolean) (SweepResult :type Hit%20Result%20Structure%20%28by%20ref%29))
  (Utilities|Casting|CastToBP_CarRollerCoaster OtherActor)
  (CallFunction|SlowEvent 4e+01))

(event OnComponentBeginOverlap(SpeedTrigger2)
  (params (OverlappedComponent :type Primitive%20Component%20Object%20Reference) (OtherActor :type Actor%20Object%20Reference) (OtherComp :type Primitive%20Component%20Object%20Reference) (OtherBodyIndex :type Integer) (bFromSweep :type Boolean) (SweepResult :type Hit%20Result%20Structure%20%28by%20ref%29))
  (Utilities|Casting|CastToBP_CarRollerCoaster OtherActor)
  (CallFunction|SpeedEvent 25.0))

(event Custom|PlayTimeLine
  (bind _spline (Variables|Default|GetSpline))
  (bind _spline_2 (Variables|Default|GetSpline))
  (bind _returnvalue (Spline|GetSplineLength _spline))
  (bind _alpha (Timeline|Timeline PlayFromStart)
    (:Update
      (for (_array_element _array_index) (Variables|Default|GetActors)
        (bind _output_get (Variables|Default|SetDistanceAlongSpline (+ (Math|Float|Lerp 0.0 (Spline|GetSplineLength (Variables|Default|GetSpline)) _alpha) (* _array_index (Variables|Default|GetOffsetbetweenActors)))))
        (if (> _output_get _returnvalue)
          (Variables|Default|SetDistanceAlongSpline (- (Variables|Default|GetDistanceAlongSpline) _returnvalue))
          (else
            (Transformation|SetActorLocationAndRotation _array_element (Spline|GetLocationatDistanceAlongSpline _spline_2 (Variables|Default|GetDistanceAlongSpline) "World") (Spline|GetRotationatDistanceAlongSpline _spline_2 (Variables|Default|GetDistanceAlongSpline) "World"))))))
    (:Finished
      (CallFunction|EndGame))))

(event Custom|EndGame
  (Game|Player|SetViewTargetwithBlend (Game|GetPlayerController 0) (Game|Player|GetPlayerPawn 0) 1.0 "VTBlend_Linear" 0.0 false)
  (bind _asmy_game_instance (Utilities|Casting|CastToMyGameInstance (Game|GetGameInstance)))
  (Default|AddCoinstoPlayer _asmy_game_instance 10)
  (Input|AddMappingContext (PlayerController|LocalPlayerSubsystems|GetEnhancedInputLocalPlayerSubsystem (Game|GetPlayerController 0)) "/Game/ThirdPerson/Input/IMC_Default.IMC_Default" 0 "(bIgnoreAllPressedKeysUntilRelease=True,bForceImmediately=False,bNotifyUserSettings=False)")
  (Variables|Default|SetplayerInGame false)
  (Default|NotificationPushEvent (Variables|Default|GetBP_Notification) "Vous venez de terminer un tour de Grand Huit!" (Utilities|Struct|MakeSlateColor "(R=0.068408,G=1.000000,B=0.000000,A=1.000000)")))

(event Custom|SlowEvent
  (params (Slow :type Float%20%28double-precision%29))
  (Variables|Default|SetSlow Slow)
  (Components|Timeline|SetPlayRate (Variables|Default|GetTimeline) (/ 1.0 (Variables|Default|GetSlow))))

(event Custom|SpeedEvent
  (params (Speed :type Float%20%28double-precision%29))
  (Variables|Default|SetSpeed Speed)
  (Components|Timeline|SetPlayRate (Variables|Default|GetTimeline) (/ 1.0 (Variables|Default|GetSpeed))))

(event Input|KeyboardEvents|E
  (params (Key :type Key%20Structure :default "None"))
  (:Pressed
    (if (Variables|Default|GetinTrigger)
      (if (not (Variables|Default|GetplayerInGame))
        (bind _asmy_game_instance (Utilities|Casting|CastToMyGameInstance (Game|GetGameInstance)))
        (if (> (Variables|/Game/Blueprints/Player/MyGameInstance.MyGameInstance_C|GetTotalTickets _asmy_game_instance) 0)
          (Variables|Default|SetplayerInGame true)
          (bind _returnvalue (Actor|GetActorOfClass "/Game/Blueprints/RollerCoaster/BP_CarRollerCoaster.BP_CarRollerCoaster_C"))
          (bind _output_get (Variables|Default|SetBP_CarRollerCoaster _returnvalue))
          (Game|Player|SetViewTargetwithBlend (Game|GetPlayerController 0) _output_get 1.0 "VTBlend_Linear" 0.0 false)
          (Input|RemoveMappingContext (PlayerController|LocalPlayerSubsystems|GetEnhancedInputLocalPlayerSubsystem (Game|GetPlayerController 0)) "/Game/ThirdPerson/Input/IMC_Default.IMC_Default" "(bIgnoreAllPressedKeysUntilRelease=True,bForceImmediately=False,bNotifyUserSettings=False)")
          (Utilities|FlowControl|Delay 1.0)
          (Components|Timeline|SetPlayRate (Variables|Default|GetTimeline) (/ 1.0 (Variables|Default|GetTimelineLength)))
          (bind _asmy_game_instance_2 (Utilities|Casting|CastToMyGameInstance (Game|GetGameInstance)))
          (Default|RemoveTicketstoPlayer _asmy_game_instance_2 1)
          (CallFunction|PlayTimeLine)
          (else
            (Default|NotificationPushEvent (Variables|Default|GetBP_Notification) "Vous n'avez pas de ticket pour faire cette attraction!" (Utilities|Struct|MakeSlateColor "(R=1.000000,G=0.120769,B=0.000000,A=1.000000)"))))))))

(fn ConstructionScript
  (bind _spline (Variables|Default|GetSpline))
  (for (_array_element _array_index) (Variables|Default|GetActors)
    (Transformation|SetActorLocationAndRotation _array_element (Spline|GetLocationatDistanceAlongSpline _spline (* (Variables|Default|GetOffsetbetweenActors) _array_index) "World") (Spline|GetRotationatDistanceAlongSpline _spline (* (Variables|Default|GetOffsetbetweenActors) _array_index) "World"))))

(fn StartPlaying
  (params (BP%20Third%20Person :type BP%20Third%20Person%20Character%20Object%20Reference))
  (Variables|Default|SetAs%20BP%20Third%20Person%20Character_0 BP%20Third%20Person)
  (|CallParentFunction BP%20Third%20Person)
  (Variables|Default|SetinTrigger true)
  (bind _returnvalue (Actor|GetActorOfClass "/Game/Blueprints/Player/BP_NotificationPush.BP_NotificationPush_C"))
  (Variables|Default|SetBP_Notification _returnvalue))