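; BP_Pause shows and hides the WG_PauseMenu widget when Backspace is pressed.
; BeginPlay hides the cursor and sets game-only input.
; Backspace checks IsOpen, which this file never sets, to either remove the stored widget and restore that state, or construct a new one with the cursor shown and mouse-locked UI-only input.
; The game itself is not paused here.
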(event EventBeginPlay
  (bind _returnvalue (Game|GetPlayerController 0))
  (Variables|/Script/Engine.PlayerController|SetbShowMouseCursor _returnvalue false)
  (Input|SetInputModeGameOnly _returnvalue false))

(event Input|KeyboardEvents|Backspace
  (params (Key :type Key%20Structure :default "None"))
  (bind _returnvalue (Game|GetPlayerController 0))
  (bind _returnvalue_2 (Game|GetPlayerController 0))
  ;[1 1 1] Open/Close Widget Pause Menu
  (:Pressed
    (if (Variables|Default|GetisOpen)
      (Widget|RemovefromParent (Variables|Default|GetPause%20Menu%20Widget))
      (Variables|/Script/Engine.PlayerController|SetbShowMouseCursor _returnvalue false)
      (Input|SetInputModeGameOnly _returnvalue false)
      (else
        (bind _returnvalue_3 (Game|ConstructObjectfromClass "/Game/Blueprints/Pause/WG_PauseMenu.WG_PauseMenu_C"))
        (bind _output_get (Variables|Default|SetPause%20Menu%20Widget _returnvalue_3))
        (UserInterface|Viewport|AddtoViewport _output_get 0)
        (Variables|/Script/Engine.PlayerController|SetbShowMouseCursor _returnvalue_2 true)
        (Input|SetInputModeUIOnly _returnvalue_2 0 "LockAlways" false)))))

(fn ConstructionScript)