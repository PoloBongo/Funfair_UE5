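; BP_NPC is a pawn that wanders between randomly chosen BP_TargetPoint actors using AI MoveTo.
; On arrival, the point's type decides the outcome: pause, spawn another NPC under a population cap, or destroy itself.
; BP_ManageNPC supplies the NPC count, and a destruction point spawns instead when that count is below one.
; Tick flags player proximity and restarts movement when the player leaves range.
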(event Custom|MoveNPC
  ;[1 1 1] Move NPC to a random target point
  (bind _output_get (Variables|Default|SetCurTargetPoint (.OutItem (Utilities|Array|Random (Variables|Default|GetOut%20Actors)))))
  (AI|AIMoveTo self (.RandomLocation (AI|Navigation|GetRandomReachablePointinRadius (Transformation|GetActorLocation _output_get) 0.0 0 0)) 0 5.0 false
    (:OnSuccess
      (switch Utilities|FlowControl|Switch|SwitchonE_NavDestinationType (Variables|/Game/Blueprints/NPC/BP_TargetPoint.BP_TargetPoint_C|GetType (Variables|Default|GetCurTargetPoint))
        (:NewEnumerator0
          (Utilities|FlowControl|Delay (Math|Random|RandomFloatinRange 2.0 6.0))
          (CallFunction|MoveNPC))
        (:NewEnumerator1
          (bind _returnvalue (Actor|GetActorOfClass "/Game/Blueprints/NPC/BP_ManageNPC.BP_ManageNPC_C"))
          (bind _output_get_2 (Variables|Default|SetManageNPC _returnvalue))
          (Default|AddNbNPC _output_get_2)
          (if (< (Variables|/Game/Blueprints/NPC/BP_ManageNPC.BP_ManageNPC_C|GetnumberOfNPC (Variables|Default|GetManageNPC)) (Variables|Default|GetmaxNPC))
            (Default|SpawnNPC (Variables|Default|GetCurTargetPoint))
            (else
              (Utilities|FlowControl|Delay 0.2)))
          (CallFunction|MoveNPC))
        (:NewEnumerator2
          (bind _returnvalue_2 (Actor|GetActorOfClass "/Game/Blueprints/NPC/BP_ManageNPC.BP_ManageNPC_C"))
          (Variables|Default|SetManageNPC _returnvalue_2)
          (if (< (Variables|/Game/Blueprints/NPC/BP_ManageNPC.BP_ManageNPC_C|GetnumberOfNPC (Variables|Default|GetManageNPC)) 1)
            (Default|SpawnNPC (Variables|Default|GetCurTargetPoint))
            (CallFunction|MoveNPC)
            (else
              (Actor|DestroyActor))))))))

(event EventBeginPlay
  ;[1 1 1] Récupère tout les targets points pour pouvoir s'y rendre plus tard
  (bind _outactors (Actor|GetAllActorsOfClass "/Game/Blueprints/NPC/BP_TargetPoint.BP_TargetPoint_C"))
  (Variables|Default|SetOut%20Actors _outactors)
  (bind _returnvalue (Actor|GetActorOfClass "/Game/ThirdPerson/Blueprints/BP_ThirdPersonCharacter.BP_ThirdPersonCharacter_C"))
  (Variables|Default|SetBP_ThirdCharacter _returnvalue)
  (CallFunction|MoveNPC))

(event EventTick
  (params (DeltaSeconds :type Float%20%28single-precision%29))
  ;[1 1 1] Check si le player est proche du NPC
  (if (<= (Math|Vector|Distance(Vector) (Transformation|GetActorLocation) (Transformation|GetActorLocation (Game|Player|GetPlayerPawn 0))) 2e+02)
    (Variables|Default|SetIsNextToPlayer true)
    (elif (Variables|Default|GetIsNextToPlayer)
      (Variables|Default|SetIsNextToPlayer false)
      (CallFunction|MoveNPC))))

(fn ConstructionScript)